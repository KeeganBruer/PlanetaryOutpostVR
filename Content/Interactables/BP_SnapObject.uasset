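; BP_SnapObject is a grabbable interactable that snaps into BP_Slot actors.
; Mesh overlaps with a slot's Box store that slot as the candidate if it is free, and clear it when the overlap ends.
; GrabComponent events attach to the stored slot on drop if it is not in use, and detach from it on grab.
; SetStatus only stores a Status value.
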(event `self.GrabComponent.OnDropped`
  (params (`Motion Controller` :type "MotionControllerComponent Object Reference"))
  (`/Engine/EditorBlueprintResources/StandardMacros.IsValid` (`self.slot`)
    (:`Is Valid`
      (if (not (`/Game/Interactables/BP_Slot.inUse` (`self.slot`)))
        (`/Game/Interactables/BP_Slot.AttachToSlot` (`self.slot`))))))

(event `self.GrabComponent.OnGrabbed`
  (params (MotionController :type "MotionControllerComponent Object Reference"))
  (`/Engine/EditorBlueprintResources/StandardMacros.IsValid` (`self.slot`)
    (:`Is Valid`
      (`/Game/Interactables/BP_Slot.DetachFromSlot` (`self.slot`)))))

(event `self.mesh.OnComponentBeginOverlap`
  (params (OverlappedComponent :type "PrimitiveComponent Object Reference") (OtherActor :type "Actor Object Reference") (OtherComp :type "PrimitiveComponent Object Reference") (OtherBodyIndex :type Integer) (bFromSweep :type Boolean) (SweepResult :type "HitResult Structure (by ref)"))
  (bind _asbp_slot (cast `/Game/Interactables/BP_Slot` OtherActor))
  (if (== (`/Game/Interactables/BP_Slot.Box` _asbp_slot) OtherComp)
    (if (not (`/Game/Interactables/BP_Slot.inUse` _asbp_slot))
      (set `self.slot` _asbp_slot))))

(event `self.mesh.OnComponentEndOverlap`
  (params (OverlappedComponent :type "PrimitiveComponent Object Reference") (OtherActor :type "Actor Object Reference") (OtherComp :type "PrimitiveComponent Object Reference") (OtherBodyIndex :type Integer))
  (`/Engine/EditorBlueprintResources/StandardMacros.IsValid` (`self.slot`)
    (:`Is Valid`
      (bind _asbp_slot (cast `/Game/Interactables/BP_Slot` OtherActor))
      (if (and (== _asbp_slot (`self.slot`)) (== (`/Game/Interactables/BP_Slot.Box` _asbp_slot) OtherComp))
        (set `self.slot` null)))))

(fn `SetStatus`
  (params (NewStatus :type String))
  (set `self.status` NewStatus))

(fn `UserConstructionScript`)