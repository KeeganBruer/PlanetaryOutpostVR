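; BP_joystick is a grabbable joystick interactable that rotates to follow the motion controller holding it.
; GrabComponent events store the controller on grab and clear it on drop.
; While held, Tick points the mesh from Base toward the controller using a look-at rotation with a yaw offset.
; It also broadcasts OnRotating with a clamped, normalized value, though that input is a constant zero rather than the computed rotation.
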(event `self.ReceiveTick`
  (params (DeltaSeconds :type "Float (single-precision)"))
  (bind _returnvalue_location (`KismetMathLibrary.BreakTransform` (`SceneComponent.K2_GetComponentToWorld` (`self.Base`))))
  (bind _motion_controller (`self.Motion Controller`)
    (:`then`
      (bind _returnvalue_location_2 (`KismetMathLibrary.BreakTransform` (`SceneComponent.K2_GetComponentToWorld` _motion_controller)))
      (bind (_returnvalue_roll _returnvalue_pitch _returnvalue_yaw) (`KismetMathLibrary.BreakRotator` (`KismetMathLibrary.FindLookAtRotation` _returnvalue_location _returnvalue_location_2)))
      (`SceneComponent.K2_SetWorldRotation` (`self.StaticMesh`) (`KismetMathLibrary.MakeRotator` (+ _returnvalue_roll 0.0) (+ _returnvalue_pitch 0.0) (+ _returnvalue_yaw 90.0)) false false)
      (`self.on Rotating` (`KismetMathLibrary.MapRangeClamped` (`KismetMathLibrary.FClamp` (+ 0.0 0.0) (`self.Min`) (`self.Max`)) (`self.Min`) (`self.Max`) 0.0 1.0)))
    (:`else`)))

(event `self.GrabComponent.OnGrabbed`
  (params (MotionController :type "MotionControllerComponent Object Reference"))
  (set `self.Motion Controller` MotionController))

(event `self.GrabComponent.OnDropped`
  (params (`Motion Controller` :type "MotionControllerComponent Object Reference"))
  (if (== `Motion Controller` (`self.Motion Controller`))
    (set `self.Motion Controller` null)))

(fn `OnRotating`
  (params (Angle :type "Float (double-precision)")))

(fn `UserConstructionScript`)