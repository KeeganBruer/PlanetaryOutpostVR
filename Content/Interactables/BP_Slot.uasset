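; BP_Slot is a snap slot that previews and accepts BP_SnapObject actors entering its box, whose extent is set at construction.
; A validity check filters objects by optional required type and status.
; The first valid overlapping object is stored and mirrored as a ghost-material mesh, then cleared when it leaves.
; AttachToSlot revalidates it, marks the slot in use and hides the ghost; DetachFromSlot reverses this.
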(event `self.Box.OnComponentBeginOverlap`
  (params (OverlappedComponent :type "PrimitiveComponent Object Reference") (OtherActor :type "Actor Object Reference") (OtherComp :type "PrimitiveComponent Object Reference") (OtherBodyIndex :type Integer) (bFromSweep :type Boolean) (SweepResult :type "HitResult Structure (by ref)"))
  (bind _asbp_snap_object (cast `/Game/Interactables/BP_SnapObject` OtherActor))
  (`self.isValidSnap` _asbp_snap_object
    (:`valid`
      (`/Engine/EditorBlueprintResources/StandardMacros.IsValid` (`self.snapObject`)
        (:`Is Not Valid`
          (bind _output_get (set `self.snapObject` _asbp_snap_object))
          (bind _mesh (`/Game/Interactables/BP_SnapObject.mesh` _output_get))
          (`StaticMeshComponent.SetStaticMesh` (`self.StaticMesh`) (`StaticMeshComponent.StaticMesh` _mesh))
          (`SceneComponent.SetWorldScale3D` (`self.StaticMesh`) (`SceneComponent.K2_GetComponentScale` _mesh))
          (`SceneComponent.SetVisibility` (`self.StaticMesh`) true false)
          (for _index (range (`PrimitiveComponent.GetNumMaterials` (`self.StaticMesh`)))
            (`PrimitiveComponent.SetMaterial` (`self.StaticMesh`) _index (`self.Ghost Material`))))))))

(event `self.Box.OnComponentEndOverlap`
  (params (OverlappedComponent :type "PrimitiveComponent Object Reference") (OtherActor :type "Actor Object Reference") (OtherComp :type "PrimitiveComponent Object Reference") (OtherBodyIndex :type Integer))
  (bind _asbp_snap_object (cast `/Game/Interactables/BP_SnapObject` OtherActor))
  (if (== _asbp_snap_object (`self.snapObject`))
    (`StaticMeshComponent.SetStaticMesh` (`self.StaticMesh`) null)
    (set `self.snapObject` null)))

(fn `AttachToSlot`
  (returns (`valid snap` :type Boolean))
  (`self.isValidSnap` (`self.snapObject`)
    (:`valid`
      (set `self.inUse` true)
      (`SceneComponent.SetVisibility` (`self.StaticMesh`) false false)
      (return true))
    (:`not Valid`
      (return false))))

(fn `DetachFromSlot`
  (returns (`valid snap` :type Boolean))
  (set `self.inUse` false)
  (`SceneComponent.SetVisibility` (`self.StaticMesh`) true false)
  (return true))

(fn `test`)

(fn `UserConstructionScript`
  (`BoxComponent.SetBoxExtent` (`self.Box`) (`self.In Box Extent`) true))